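; Segment actor for a snake chain that calls ConstrainDistance against its NextSection every tick, in what appears to be a constraints programming demo.
; Construction uses the section's index relative to total size to shade a dynamic material and taper scale toward half size.
; An angle constraint call exists but is unwired.
; A separate helper, not called here, clamps jump velocity to a cone around a surface normal, preserving magnitude.
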(event `self.ReceiveTick`
  (params (DeltaSeconds :type "Float (single-precision)"))
  (`self.ConstrainDistance` (`self.NextSection`)))

(fn `ClampJumpDirectionAroundNormal`
  (params (JumpVelocity :type "Vector Structure") (SurfaceNormal :type "Vector Structure") (ConeAngle :type "Float (double-precision)"))
  (returns (NewJumpVelocity :type "Vector Structure"))
  (return (`KismetMathLibrary.SelectVector` (`local.JumpVelocity`) (* (`KismetMathLibrary.RotateAngleAxis` (`local.SurfaceNormal`) (`local.ConeAngle`) (`KismetMathLibrary.Cross_VectorVector` (`local.JumpVelocity`) (`local.SurfaceNormal`))) (`KismetMathLibrary.VSize` (`local.JumpVelocity`))) (< (`KismetMathLibrary.DegAcos` (`KismetMathLibrary.Dot_VectorVector` (`KismetMathLibrary.Normal` (`local.JumpVelocity`)) (`local.SurfaceNormal`))) (`local.ConeAngle`)))))

(fn `UserConstructionScript`
  (bind _returnvalue (`PrimitiveComponent.CreateDynamicMaterialInstance` (`self.StaticMeshComponent`) 0 "/ProceduralAnimation/Constraints/Programming/MI_Section.MI_Section" "None"))
  (bind _output_get (set `self.Mat` _returnvalue))
  (`MaterialInstanceDynamic.SetVectorParameterValue` _output_get "Color" (`KismetMathLibrary.Conv_DoubleToLinearColor` (`KismetSystemLibrary.MakeLiteralDouble` (/ (`KismetMathLibrary.Conv_IntToDouble` (`self.SectionIndex`)) (`KismetMathLibrary.Conv_IntToDouble` (`self.TotalSize`))))))
  (`self.SetActorScale3D` (`KismetMathLibrary.Conv_DoubleToVector` (`KismetMathLibrary.MapRangeClamped` (/ (`KismetMathLibrary.Conv_IntToDouble` (`self.SectionIndex`)) (`KismetMathLibrary.Conv_IntToDouble` (`self.TotalSize`))) 0.0 1.0 1.0 0.5))))