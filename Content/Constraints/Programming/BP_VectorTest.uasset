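; BP_VectorTest is a debug actor that visualizes a vector cross product.
; Every Tick it draws a red arrow from the actor to StaticMesh1 and a blue arrow to StaticMesh.
; A green arrow shows the cross product of the two meshes' relative locations, offset from the actor's position, so moving either mesh changes the result.
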(event `self.ReceiveTick`
  (params (DeltaSeconds :type "Float (single-precision)"))
  (bind _returnvalue (`self.K2_GetActorLocation`))
  (`KismetSystemLibrary.DrawDebugArrow` (`self.K2_GetActorLocation`) (`SceneComponent.K2_GetComponentLocation` (`self.StaticMesh1`)) 0.0 (struct :`R` 1.0 :`B` 0.017204 :`A` 1.0) 0.0 4.0)
  (`KismetSystemLibrary.DrawDebugArrow` (`self.K2_GetActorLocation`) (`SceneComponent.K2_GetComponentLocation` (`self.StaticMesh`)) 0.0 (struct :`G` 0.117884 :`B` 1.0 :`A` 1.0) 0.0 4.0)
  (`KismetSystemLibrary.DrawDebugArrow` _returnvalue (+ _returnvalue (`KismetMathLibrary.Cross_VectorVector` (`SceneComponent.RelativeLocation` (`self.StaticMesh1`)) (`SceneComponent.RelativeLocation` (`self.StaticMesh`)))) 0.0 (struct :`R` 0.019072 :`G` 1.0 :`A` 1.0) 0.0 4.0))

(fn `UserConstructionScript`)