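; BP_Snake is a snake actor that builds itself on BeginPlay as a chain of BP_Snake_Section actors.
; CreateSections spawns evenly spaced sections along world X, passing each its index, the total count, and distance and angle constraints.
; Sections form a doubly linked list through NextSection and PrevSection, with the first becoming Head, snapped and attached to the snake.
; Tick and turn input are empty, leaving head movement and rotation code disconnected.
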(event `self.ReceiveBeginPlay`
  (`parent.ReceiveBeginPlay`)
  (`self.CreateSections` (`self.Sections`)))

(event `self.ReceiveTick`
  (params (DeltaSeconds :type "Float (single-precision)")))

(event `EnhancedInput|/ProceduralAnimation/Constraints/Programming/Framework/IA_TurnRight`
  (params (ActionValue :type "Float (double-precision)") (ElapsedSeconds :type "Float (double-precision)") (TriggeredSeconds :type "Float (double-precision)") (InputAction :type "InputAction Object Reference" :default "/ProceduralAnimation/Constraints/Programming/Framework/IA_TurnRight.IA_TurnRight")))

(fn `CreateSections`
  (params (NumSections :type Integer))
  (locals (L_TempIdx :type Integer) (L_NewSection :type "SnakeSection Object Reference") (L_Curr :type "SnakeSection Object Reference"))
  (bind (_returnvalue_location _returnvalue_rotation _returnvalue_scale) (`KismetMathLibrary.BreakTransform` (`self.GetTransform`)))
  (`parent.CreateSections` NumSections)
  (for _index (range NumSections)
    (bind _output_get (set `local.L_TempIdx` _index))
    (bind _returnvalue (`|SpawnActorFromClass` "/ProceduralAnimation/Constraints/Programming/BP_Snake_Section.BP_Snake_Section_C" (`KismetMathLibrary.MakeTransform` (+ _returnvalue_location (`KismetMathLibrary.MakeVector` (`KismetMathLibrary.Conv_IntToDouble` (* _output_get 100)))) _returnvalue_rotation _returnvalue_scale) "Undefined" "MultiplyWithRoot" null (`local.L_TempIdx`) (`local.NumSections`) (`self.DistanceConstraint`) (`self.AngleConstraint`) null))
    (set `local.L_NewSection` _returnvalue)
    (`local.L_Curr`
      (:`then`
        (set `/ProceduralAnimation/Constraints/Programming/BP_Snake_Section.NextSection` (`local.L_NewSection`) (`local.L_Curr`))
        (set `/ProceduralAnimation/Constraints/Programming/BP_Snake_Section.PrevSection` (`local.L_Curr`) (`local.L_NewSection`))
        (set `local.L_Curr` (`local.L_NewSection`)))
      (:`else`
        (bind _output_get_2 (set `local.L_Curr` (`local.L_NewSection`)))
        (bind _output_get_3 (set `self.Head` _output_get_2))
        (`self.K2_AttachToActor` _output_get_3 self "None" "SnapToTarget" "SnapToTarget" "SnapToTarget" true)))))

(fn `UserConstructionScript`)