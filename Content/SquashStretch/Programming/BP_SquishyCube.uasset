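; BP_SquishyCube is a physics test actor, apparently for squash-and-stretch work, though this Blueprint holds no active deformation logic.
; It records its start location on BeginPlay, and a looping timer periodically moves it back there and zeroes the StaticMesh's linear and angular velocity.
; Tick prints the actor's velocity on screen, and an actor-scale node is left unconnected.
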(event `self.ReceiveBeginPlay`
  (set `self.StartLocation` (`self.K2_GetActorLocation`))
  (`KismetSystemLibrary.K2_SetTimerDelegate` (delegate `Reset`) 4.0 true))

(event `Reset`
  (bind _staticmesh (`self.StaticMesh`))
  (`self.K2_SetActorTransform` (`KismetMathLibrary.MakeTransform` (`self.StartLocation`)))
  (`PrimitiveComponent.SetPhysicsLinearVelocity` _staticmesh (0.0 0.0 0.0) false "None")
  (`PrimitiveComponent.SetPhysicsAngularVelocityInDegrees` _staticmesh (0.0 0.0 0.0) false "None"))

(event `self.ReceiveTick`
  (params (DeltaSeconds :type "Float (single-precision)"))
  (`KismetSystemLibrary.PrintText` (`KismetTextLibrary.Conv_VectorToText` (`self.GetVelocity`)) true false (struct :`G` 0.66 :`B` 1.0 :`A` 1.0) 0.0))

(fn `UserConstructionScript`)